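; BP_TestGameMode is a test game mode that paints a 2D metaball image into a memory texture in Blueprint.
; On OnStartBlueprintFill, it visits every pixel and sums each ball's inverse squared, radius-scaled distance, substituting the radius at exact centers to avoid dividing by zero.
; Pixels whose influence exceeds the Border setting get the light color, others the dark, then the texture is applied once.
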(event EventOnStartBlueprintFill
  (params (MemTexture :type Memory%20Texture%20Object%20Reference) (Settings :type Test%20Settings%20Object%20Reference) (Balls :type Array%20of%20Meta%20Ball%20Object%20References))
  ;[1 1 1] For Each Pixel
  (for _index (range 0 (Class|MemoryTexture|GetWidth MemTexture))
    (for _index_2 (range 0 (Class|MemoryTexture|GetHeight MemTexture))
      ;[1 1 1] Foreach Pixels Influence
      (Variables|Default|SetInfluence 0.0)
      (for _array_element Balls
        (if (and (== _index (Variables|/Script/SpeedTestUnreal.MetaBall|GetX _array_element)) (== _index_2 (Variables|/Script/SpeedTestUnreal.MetaBall|GetY _array_element)))
          (Variables|Default|SetInfluence (+ (Variables|Default|GetInfluence) (Variables|/Script/SpeedTestUnreal.MetaBall|GetR _array_element)))
          (else
            (Variables|Default|SetInfluence (+ (/ 1.0 (+ (Math|Float|Power (/ (- _index (Variables|/Script/SpeedTestUnreal.MetaBall|GetX _array_element)) (Variables|/Script/SpeedTestUnreal.MetaBall|GetR _array_element)) 2.0) (Math|Float|Power (/ (- _index_2 (Variables|/Script/SpeedTestUnreal.MetaBall|GetY _array_element)) (Variables|/Script/SpeedTestUnreal.MetaBall|GetR _array_element)) 2.0))) (Variables|Default|GetInfluence))))))
      ;[1 1 1] Set Pixel Color
      (if (> (Variables|Default|GetInfluence) (Variables|/Script/SpeedTestUnreal.TestSettings|GetBorder Settings))
        (Class|MemoryTexture|SetPixel MemTexture (Variables|/Script/SpeedTestUnreal.TestSettings|GetLightColor Settings) _index _index_2)
        (else
          (Class|MemoryTexture|SetPixel MemTexture (Variables|/Script/SpeedTestUnreal.TestSettings|GetDarkColor Settings) _index _index_2)))))
  (Class|MemoryTexture|Apply MemTexture))

(fn ConstructionScript)